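; Player controller for Player 1 in what appears to be a card game, handling the HUD and pause screen toggle.
; BeginPlay adds the Player 1 HUD to the viewport and shows the mouse cursor.
; The pause input lazily creates the pause widget, then toggles its visibility, switching cursor and input mode between game-and-UI and game-only.
; The game itself is never paused here.
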(event `self.ReceiveBeginPlay`
  (bind _returnvalue (`|CreateWidget` "/Game/_CardUI/W_Player1HUD.W_Player1HUD_C" self))
  (`UserWidget.AddToViewport` _returnvalue 0)
  (set `self.bShowMouseCursor` true))

(event `InputAction|Toggle_Game_Pause`
  (params (Key :type "Key Structure"))
  ;[0.0107 1 0] Toggle/Pause Screen
  (:`Pressed`
    (`self.Toggle_pause`)))

(fn `Focus Game`
  (set `self.bShowMouseCursor` false)
  (`WidgetBlueprintLibrary.SetInputMode_GameOnly` self))

(fn `Focus_widget`
  (set `self.bShowMouseCursor` true)
  (`WidgetBlueprintLibrary.SetInputMode_GameAndUIEx` self (`self.Game_Paused`)))

(fn `Toggle_pause`
  (`self.Game_Paused`
    (:`then`
      (if (`Widget.IsVisible` (`self.Game_Paused`))
        (`Widget.SetVisibility` (`self.Game_Paused`) "Collapsed")
        (`self.Focus Game`)
        (else
          (`Widget.SetVisibility` (`self.Game_Paused`) "Visible")
          (`self.Focus_widget`))))
    (:`else`
      (bind _returnvalue (`|CreateWidget` "/Game/_Noah/widgets/Pause_Screen.Pause_Screen_C" self))
      (bind _output_get (set `self.Game_Paused` _returnvalue))
      (`UserWidget.AddToViewport` _output_get 0)
      (`self.Focus_widget`))))

(fn `UserConstructionScript`)