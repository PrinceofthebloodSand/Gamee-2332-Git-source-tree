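; Game Instance Blueprint that handles session teardown for a multiplayer game.
; Travel and network error events print the failure type, then share a call that destroys the session through player controller 0.
; A LeaveSession event opens the main menu level and then destroys the session.
; Init and Shutdown are empty.
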(event `self.ReceiveShutdown`)

(event `self.ReceiveInit`)

(event `self.HandleTravelError`
  (params (FailureType :type "ETravelFailure Enum" :default "NoLevel"))
  ;[1 0 0.0553] Handlieng error
  (`KismetSystemLibrary.PrintString` (`|GetEnumeratorNameAsString` FailureType) true true (struct :`R` 0.770833 :`G` 0.007288 :`A` 1.0) 5.0)
  (`DestroySessionCallbackProxy.DestroySession` (`GameplayStatics.GetPlayerController` 0) :!label _label))

(event `self.HandleNetworkError`
  (params (FailureType :type "ENetworkFailure Enum" :default "NetDriverAlreadyExists") (bIsServer :type Boolean))
  ;[1 0 0.0553] Handlieng error
  (`KismetSystemLibrary.PrintString` (`|GetEnumeratorNameAsString` FailureType) true true (struct :`R` 1.0 :`B` 0.022033 :`A` 1.0) 5.0)
  (goto _label))

(event `LeaveSession`
  ;[0.3204 0 1] Leave_Session
  (`GameplayStatics.OpenLevel` "Main_Menu_Level")
  (`DestroySessionCallbackProxy.DestroySession` (`GameplayStatics.GetPlayerController` 0)))